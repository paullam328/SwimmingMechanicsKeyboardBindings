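; Prototype player character with a gun attached to its hands, handling movement, look, sprint, crouch, jump and swimming through input axes and custom events.
; BeginPlay creates the HUD widget.
; While the MyPlayer controller is not sprinting, Tick resets walk speed and, if interaction is enabled, updates compass rotation and traces from the camera.
; The trace sends hover messages when its target changes; customInteract is empty and the interact message call is unconnected.
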(event `customMoveForward`
  (params (AxisValue :type "Float (double-precision)"))
  ;[1 1 1] Base
  ;;[1 1 1] Movement
  (`self.AddMovementInput` (`self.GetActorForwardVector`) AxisValue))

(event `customMoveRight`
  (params (AxisValue :type "Float (double-precision)"))
  ;[1 1 1] Base
  ;;[1 1 1] Movement
  (`self.AddMovementInput` (`self.GetActorRightVector`) AxisValue))

(event `InputAxis|MoveForward`
  (params (AxisValue :type "Float (single-precision)"))
  ;[1 1 1] Base
  ;;[1 1 1] Movement
  (if (not (`self.MovementDisabled`))
    (`self.AddMovementInput` (`self.GetActorForwardVector`) AxisValue)))

(event `InputAxis|MoveRight`
  (params (AxisValue :type "Float (single-precision)"))
  ;[1 1 1] Base
  ;;[1 1 1] Movement
  (if (not (`self.MovementDisabled`))
    (`self.AddMovementInput` (`self.GetActorRightVector`) AxisValue)))

(event `customLookUp`
  (params (AxisValue :type "Float (double-precision)"))
  ;[1 1 1] Base
  ;;[1 1 1] Looking
)

(event `InputAxis|LookUp`
  (params (AxisValue :type "Float (single-precision)"))
  ;[1 1 1] Base
  ;;[1 1 1] Looking
  (if (not (`self.LookingDisabled`))
    (`self.AddControllerPitchInput` (* AxisValue (`self.MouseSensitivity`)))))

(event `InputAxis|Turn`
  (params (AxisValue :type "Float (single-precision)"))
  ;[1 1 1] Base
  ;;[1 1 1] Looking
  (if (not (`self.LookingDisabled`))
    (`self.AddControllerYawInput` (* AxisValue (`self.MouseSensitivity`)))))

(event `customSprint`
  (params (isSprinting :type Boolean))
  (bind _charactermovement (`self.CharacterMovement`))
  ;[1 1 1] Actions
  ;;[1 1 1] Running
  (if true
    (set `self.RunPressed` true)
    (set `CharacterMovementComponent.MaxWalkSpeed` 375.0 _charactermovement)
    (else
      (set `self.RunPressed` false)
      (if (`self.CrouchPressed`)
        (set `CharacterMovementComponent.MaxWalkSpeed` 160.0 _charactermovement)
        (else
          (set `CharacterMovementComponent.MaxWalkSpeed` 200.0 _charactermovement))))))

(event `InputAction|Run`
  (params (Key :type "Key Structure"))
  ;[1 1 1] Actions
  ;;[1 1 1] Running
)

(event `InputAction|Crouch`
  (params (Key :type "Key Structure"))
  ;[1 1 1] Actions
  ;;[1 1 1] Crouching
)

(event `customCrouch`
  (bind _charactermovement (`self.CharacterMovement`))
  ;[1 1 1] Actions
  ;;[1 1 1] Crouching
  (`/Engine/EditorBlueprintResources/StandardMacros.FlipFlop`
    (:`A`
      (set `self.CrouchPressed` true)
      (set `CharacterMovementComponent.MaxWalkSpeed` 160.0 _charactermovement))
    (:`B`
      (set `self.CrouchPressed` false)
      (if (`self.RunPressed`)
        (set `CharacterMovementComponent.MaxWalkSpeed` 375.0 _charactermovement)
        (else
          (set `CharacterMovementComponent.MaxWalkSpeed` 200.0 _charactermovement))))))

(event `customJump`
  ;[1 1 1] Actions
  ;;[1 1 1] Jumping
  (if (`NavMovementComponent.IsSwimming` (`self.CharacterMovement`))
    _
    (elif (not (`self.MovementDisabled`))
      (`self.Jump`)
      (set `self.JumpPressed` true))))

(event `self.ReceiveBeginPlay`
  ;[1 1 1] Creating and Adding HUD Widget to Player Screen
  (bind _returnvalue (`|CreateWidget` "/Game/Prototype/UI/Blueprints/BP_HeadsUpDisplay_PROTNew.BP_HeadsUpDisplay_PROTNew_C"))
  (bind _output_get (set `self.HeadsUpDisplay` _returnvalue))
  (`UserWidget.AddToViewport` _output_get 0))

(event `InputAxis|SwimUp`
  (params (AxisValue :type "Float (single-precision)"))
  ;[1 1 1] Actions
  ;;[1 1 1] Swimming
  (if (`NavMovementComponent.IsSwimming` (`self.CharacterMovement`))
    (`self.AddMovementInput` (`KismetMathLibrary.GetUpVector` (`KismetMathLibrary.MakeRotator` 0.0 0.0 (.yaw (`self.GetControlRotation`)))) AxisValue)))

(event `InputAction|Interact`
  (params (Key :type "Key Structure")))

(event `customInteract`
  ;[1 1 1] Interact
)

(event `customSwimUp`
  (params (AxisValue :type "Float (double-precision)"))
  ;[1 1 1] Actions
  ;;[1 1 1] Swimming
  (`self.AddMovementInput` (`KismetMathLibrary.GetUpVector` (`KismetMathLibrary.MakeRotator` 0.0 0.0 (.yaw (`self.GetControlRotation`)))) AxisValue))

(event `self.ReceiveTick`
  (params (DeltaSeconds :type "Float (single-precision)"))
  (bind (_returnvalue_roll _returnvalue_pitch _returnvalue_yaw) (`KismetMathLibrary.BreakRotator` (`self.K2_GetActorRotation`)))
  ;[1 1 1] SetWalkingSpeed
  (bind _asmy_player (cast `/Game/Maps/Dev/MyPlayer` (`GameplayStatics.GetPlayerController` 0)))
  (if (not (`/Game/Maps/Dev/MyPlayer.sprintPressed` _asmy_player))
    (set `CharacterMovementComponent.MaxWalkSpeed` 200.0 (`self.CharacterMovement`))
    ;[1 1 1] Line Tracing
    (if (not (`self.InteractionDisabled`))
      (`self.LineTrace`) ; Line trace optimization
      (set `self.CompassRotation` _returnvalue_yaw))))

(fn `LineTrace`
  (bind _camera (`self.Camera`))
  (bind _traceactor (`self.TraceActor`))
  (bind _headsupdisplay (`self.HeadsUpDisplay`))
  (bind _returnvalue (`SceneComponent.K2_GetComponentLocation` _camera))
  (bind _outhit (`KismetSystemLibrary.LineTraceSingle` _returnvalue (+ _returnvalue (* (`KismetMathLibrary.GetForwardVector` (`SceneComponent.K2_GetComponentRotation` _camera)) (`self.InteractionDistance`))) "TraceTypeQuery1"))
  (bind (_bblockinghit _binitialoverlap _time _distance _location _impactpoint _normal _impactnormal _physmat _hitactor) (`GameplayStatics.BreakHitResult` _outhit))
  (set `self.HitPoint` _impactpoint)
  (if (!= _traceactor _hitactor)
    (message `/Game/Prototype/Gameplay/Blueprints/BP_InteractionInterface.Hover` _traceactor _headsupdisplay)
    (bind _output_get (set `self.TraceActor` _hitactor))
    (message `/Game/Prototype/Gameplay/Blueprints/BP_InteractionInterface.Hover` _output_get _headsupdisplay)))

(fn `SetLaserVisibility`
  (params (Visibility :type Boolean))
  (`SceneComponent.SetVisibility` (`self.Laser`) Visibility false))

(fn `UserConstructionScript`
  (`SceneComponent.K2_AttachToComponent` (`self.Gun`) (`self.Hands`) "GripPoint" "SnapToTarget" "SnapToTarget" "SnapToTarget" true))