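; Prototype mineable actor that loses durability as it is mined and is pulled into the player when depleted.
; Tick polls the player controller's InteractPressed; while true, it calls Interact and Hover, shows sparks at the player's hit point and toggles a gate.
; The open gate decrements Durability per tick.
; At zero, a timeline moves the actor to the player while shrinking it, then shows a HUD notification and destroys it.
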(event `self.ReceiveTick`
  (params (DeltaSeconds :type "Float (single-precision)"))
  (bind _sparks (`self.Sparks`))
  (bind _durability (`self.Durability`))
  (`|ExecutionSequence`
    (:`then_0`
      ;[1 1 1] Actor Tick
      (`/Engine/EditorBlueprintResources/StandardMacros.Gate` true :!label _label
        (:`Exit`
          ;;[1 1 1] Branch will fire only once
          (`/Engine/EditorBlueprintResources/StandardMacros.DecrementInt` _durability
            (:`  `
              (if (== _durability 0)
                (`SceneComponent.SetVisibility` (`self.Sparks`) false false)
                (bind _output_get (set `self.ActorStartLocation` (`self.K2_GetActorLocation`)))
                (bind (_direction _alpha) (`Timeline|Timeline_0` :!via `PlayFromStart`)
                  (:`Update`
                    ;;[1 1 1] Sweep Animation Update
                    (`self.K2_SetActorLocation` (`KismetMathLibrary.VLerp` _output_get (`self.K2_GetActorLocation` (`GameplayStatics.GetPlayerPawn` 0)) _alpha))
                    (`SceneComponent.SetWorldScale3D` (`self.StaticMesh`) (`KismetMathLibrary.VLerp` (1.0 1.0 1.0) (0.0 0.0 0.0) _alpha)))
                  (:`Finished`
                    (bind _headsupdisplay (`/Game/Prototype/Characters/Player/Blueprints/BP_PlayerCharacter_PROT.HeadsUpDisplay` (stale _asbp_player_character_prot)))
                    ;[1 1 1] Sweep Animation Finished
                    (`/Game/Prototype/UI/Blueprints/BP_HeadsUpDisplay_PROTNew.ShowNotification` _headsupdisplay)
                    (`self.K2_DestroyActor`)))))))))
    (:`then_1`
      (bind _asbp_player_character_prot (cast `/Game/Prototype/Characters/Player/Blueprints/BP_PlayerCharacter_PROT` (`GameplayStatics.GetPlayerCharacter` 0)))
      (bind _asmy_player (cast `/Game/Maps/Dev/MyPlayer` (`GameplayStatics.GetPlayerController` 0)))
      (if (`/Game/Maps/Dev/MyPlayer.interactPressed` _asmy_player)
        (`|ExecutionSequence`
          (:`then_0`
            (bind _hitpoint (`/Game/Prototype/Characters/Player/Blueprints/BP_PlayerCharacter_PROT.HitPoint` _asbp_player_character_prot))
            (`self.Interact` _headsupdisplay _hitpoint)
            (`SceneComponent.K2_SetWorldLocation` _sparks _hitpoint false false)
            (`SceneComponent.SetVisibility` _sparks true false)
            (goto _label :!via `Toggle`))
          (:`then_1`
            ;[1 1 1] Hover Parent Function
            (`self.Hover` _headsupdisplay)
            (`parent.Hover` null)))))))

(fn `UserConstructionScript`
  (`parent.UserConstructionScript`))